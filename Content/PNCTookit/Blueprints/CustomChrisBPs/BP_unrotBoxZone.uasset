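; BP_unrotBoxZone is a trigger zone that reduces the player's rot points while they are inside, judging by its event names.
; Actor begin and end overlap identify the player by comparing the display name to BP_PNCCharacter_3D_Player.
; It fetches the first RotPointsWidget on each overlap, calling its decrease event on entry and its increase event on exit.
; The zone holds no rot state itself, leaving that logic to the widget.
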(event `self.ReceiveBeginPlay`)

(event `self.ReceiveActorBeginOverlap`
  (params (OtherActor :type "Actor Object Reference"))
  (if (`KismetStringLibrary.EqualEqual_StrStr` (`KismetSystemLibrary.GetDisplayName` OtherActor) "BP_PNCCharacter_3D_Player")
    (bind _foundwidgets (`WidgetBlueprintLibrary.GetAllWidgetsOfClass` "/Game/PNCTookit/Blueprints/Widgets/CustomChris/rotPointsWidget.rotPointsWidget_C" false))
    (`/Game/PNCTookit/Blueprints/Widgets/CustomChris/rotPointsWidget.decreaseRotPoints_Event` (`|GetArrayItem` _foundwidgets))))

(event `self.ReceiveActorEndOverlap`
  (params (OtherActor :type "Actor Object Reference"))
  (if (`KismetStringLibrary.EqualEqual_StrStr` (`KismetSystemLibrary.GetDisplayName` OtherActor) "BP_PNCCharacter_3D_Player")
    (bind _foundwidgets (`WidgetBlueprintLibrary.GetAllWidgetsOfClass` "/Game/PNCTookit/Blueprints/Widgets/CustomChris/rotPointsWidget.rotPointsWidget_C" false))
    (`/Game/PNCTookit/Blueprints/Widgets/CustomChris/rotPointsWidget.eventInreaseRotPoints_Event` (`|GetArrayItem` _foundwidgets))))

(fn `UserConstructionScript`)