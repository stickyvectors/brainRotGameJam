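; BP_unrotZone is a zone actor that relieves rot on the player while the player is inside it.
; When BP_PNCCharacter_3D_Player begins overlapping, it triggers the decrease event on RotPointsWidget; when the overlap ends, it triggers the increase event.
; It holds no rot state, reaching the widget by searching top-level widgets on each overlap and using the first result unchecked.
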(event `self.ReceiveBeginPlay`)

(event `self.ReceiveActorBeginOverlap`
  (params (OtherActor :type "Actor Object Reference"))
  (if (== OtherActor "/Game/PNCTookit/Blueprints/Characters/3D/BP_PNCCharacter_3D_Player.BP_PNCCharacter_3D_Player")
    (bind _foundwidgets (`WidgetBlueprintLibrary.GetAllWidgetsOfClass` "/Game/PNCTookit/Blueprints/Widgets/CustomChris/rotPointsWidget.rotPointsWidget_C"))
    (`/Game/PNCTookit/Blueprints/Widgets/CustomChris/rotPointsWidget.decreaseRotPoints_Event` (`|GetArrayItem` _foundwidgets))))

(event `self.ReceiveActorEndOverlap`
  (params (OtherActor :type "Actor Object Reference"))
  (if (== OtherActor "/Game/PNCTookit/Blueprints/Characters/3D/BP_PNCCharacter_3D_Player.BP_PNCCharacter_3D_Player")
    (bind _foundwidgets (`WidgetBlueprintLibrary.GetAllWidgetsOfClass` "/Game/PNCTookit/Blueprints/Widgets/CustomChris/rotPointsWidget.rotPointsWidget_C"))
    (`/Game/PNCTookit/Blueprints/Widgets/CustomChris/rotPointsWidget.eventInreaseRotPoints_Event` (`|GetArrayItem` _foundwidgets))))

(fn `UserConstructionScript`)