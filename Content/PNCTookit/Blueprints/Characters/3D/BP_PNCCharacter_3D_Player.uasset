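; 3D player character Blueprint for the PNC toolkit that adds partial physics simulation to its skeletal mesh.
; On BeginPlay it enables physics on all bodies below a configurable bone, excluding the bone itself, and initializes their blend weight.
; Despite its rotation-related name, increaseRot_Event sets that physics blend weight from the passed value, controlling how much simulation overrides animation.
; The construction script only calls its parent.
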(event `self.ReceiveBeginPlay`
  (bind _bone (`self.bone`))
  (`SkeletalMeshComponent.SetAllBodiesBelowSimulatePhysics` (`self.Mesh`) (`KismetStringLibrary.Conv_StringToName` _bone) true false)
  (`SkeletalMeshComponent.SetAllBodiesBelowPhysicsBlendWeight` (`self.Mesh`) (`KismetStringLibrary.Conv_StringToName` _bone) 0.0 false true))

(event `increaseRot_Event`
  (params (newRotValue :type "Float (double-precision)"))
  (`SkeletalMeshComponent.SetAllBodiesBelowPhysicsBlendWeight` (`self.Mesh`) (`KismetStringLibrary.Conv_StringToName` (`self.bone`)) newRotValue false true))

(fn `UserConstructionScript`
  (`parent.UserConstructionScript`))